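; Fish boss enemy that guards one of two crystals, chosen by BossIndex, and removes itself, its block and camera trigger at BeginPlay if that crystal is already owned.
; Tick drives chasing, starts a random tail or front attack when the player is in range, and polls hitbox overlaps during Delay-timed damage windows.
; Hits via BPCDamagable cost one HP with brief invulnerability; death releases the BP_BossBlock and spawns the crystal.
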(event `self.ReceiveBeginPlay`
  (bind _asbp_player (cast `/Game/GAME/BP/BP_Player` (`GameplayStatics.GetPlayerPawn` 0)))
  (set `self.As BP Player` _asbp_player)
  (`SceneComponent.SetVisibility` (`self.TailHitBox`) false false)
  (`SceneComponent.SetVisibility` (`self.FrontHitBox`) false false)
  (add `/Game/GAME/BP/Components/BPC_Damagable.TakeDamageCall` (`self.BPC_Damagable`) (delegate `Take Damage`))
  (bind _asbp_game_instance (cast `/Game/GAME/BP/BP_GameInstance` (`GameplayStatics.GetGameInstance`)))
  (set `self.As BP Game Instance` _asbp_game_instance)
  (if (`self.BossIndex`)
    (if (`/Game/GAME/BP/BP_GameInstance.HasSecondCrystal?` _asbp_game_instance)
      (bind _outactors (`GameplayStatics.GetAllActorsOfClass` "/Game/GAME/BP/Manager/BP_BossBlock.BP_BossBlock_C" :!label _label))
      (`self.K2_DestroyActor` (`|GetArrayItem` _outactors))
      (bind _outactors_2 (`GameplayStatics.GetAllActorsOfClass` "/Game/GAME/BP/Manager/Bp_TriggerBossCam.Bp_TriggerBossCam_C"))
      (`self.K2_DestroyActor` (`|GetArrayItem` _outactors_2))
      (`self.K2_DestroyActor`))
    (elif (`/Game/GAME/BP/BP_GameInstance.HasFirstCrystal?` _asbp_game_instance)
      (goto _label))))

(event `Take Damage`
  (bind _bpc_damagable (`self.BPC_Damagable`))
  (bind _capsulecomponent (`self.CapsuleComponent`))
  (bind _returnvalue (`SceneComponent.K2_GetComponentLocation` _capsulecomponent))
  (bind _returnvalue_2 (- (`/Game/GAME/BP/Components/BPC_Damagable.Hp` _bpc_damagable) 1))
  (if (not (`self.Is Undammageable ?`))
    (if (> _returnvalue_2 0)
      (set `self.Is Undammageable ?` true)
      (`GameplayStatics.PlaySound2D` "/Game/GAME/SOUND/SOUNDEFFECT/Sword_Slash_-_Sound_Effect_HD.Sword_Slash_-_Sound_Effect_HD" 1.0 1.0 0.6 null null)
      (`self.PlayAnimMontage` "/Game/GAME/ASSETS/ENNEMIES/Boss/ANim/FishBoss_Hit_Armature_Hit_Montage.FishBoss_Hit_Armature_Hit_Montage")
      (bind _output_get (set `/Game/GAME/BP/Components/BPC_Damagable.Hp` _returnvalue_2 _bpc_damagable))
      (`KismetSystemLibrary.PrintString` (`KismetStringLibrary.Conv_IntToString` _output_get))
      (`KismetSystemLibrary.Delay` 0.6)
      (set `self.Is Undammageable ?` false)
      (elif (not (`self.Is dead`))
        (set `self.Is dead` true)
        (set `self.TailDoDamage?` false)
        (set `self.FrontDoDamage?` false)
        (`PrimitiveComponent.SetCollisionEnabled` _capsulecomponent "NoCollision")
        (bind _outactors (`GameplayStatics.GetAllActorsOfClass` "/Game/GAME/BP/Manager/BP_BossBlock.BP_BossBlock_C"))
        (`/Game/GAME/BP/Manager/BP_BossBlock.Release` (`|GetArrayItem` _outactors))
        (if (`self.BossIndex`)
          (`|SpawnActorFromClass` "/Game/GAME/BP/BP_PROPS/Bp_Crystal2.Bp_Crystal2_C" (`KismetMathLibrary.MakeTransform` _returnvalue (struct) (0.3 0.3 0.3)) "Undefined" "MultiplyWithRoot" null null)
          (else
            (`|SpawnActorFromClass` "/Game/GAME/BP/BP_PROPS/Bp_Crystal1.Bp_Crystal1_C" (`KismetMathLibrary.MakeTransform` _returnvalue (struct) (0.3 0.3 0.3)) "Undefined" "MultiplyWithRoot" null null)))))))

(event `self.ReceiveTick`
  (params (DeltaSeconds :type "Float (single-precision)"))
  (if (not (`self.Is dead`))
    (`|ExecutionSequence`
      (:`then_0`
        (if (`self.Follow Player`)
          (`self.AddMovementInput` (- (`self.K2_GetActorLocation` (`self.As BP Player`)) (`self.K2_GetActorLocation`)))))
      (:`then_1`
        (`/Engine/EditorBlueprintResources/StandardMacros.IsValid` (`|GetArrayItem` (`PrimitiveComponent.GetOverlappingActors` (`self.Sphere`) "/Game/GAME/BP/BP_Player.BP_Player_C"))
          (:`Is Valid`
            (if (`self.Can Attack`)
              (`self.ChooseAttack`)))))
      (:`then_2`
        (if (`self.TailDoDamage?`)
          (for _array_element (`PrimitiveComponent.GetOverlappingActors` (`self.TailHitBox`) null)
            (`/Engine/EditorBlueprintResources/StandardMacros.IsValid` (`self.GetComponentByClass` _array_element "/Game/GAME/BP/Components/BPC_Player.BPC_Player_C")
              (:`Is Valid`
                (`KismetSystemLibrary.PrintString` "Hello")
                (set `self.TailDoDamage?` false)
                (`/Game/GAME/BP/BP_Player.TakeDamage` (`self.As BP Player`) (`/Game/GAME/BP/Components/BPC_Damagable.Damage` (`self.BPC_Damagable`))))))))
      (:`then_3`
        (if (`self.FrontDoDamage?`)
          (for _array_element_2 (`PrimitiveComponent.GetOverlappingActors` (`self.FrontHitBox`) null)
            (`/Engine/EditorBlueprintResources/StandardMacros.IsValid` (`self.GetComponentByClass` _array_element_2 "/Game/GAME/BP/Components/BPC_Player.BPC_Player_C")
              (:`Is Valid`
                (`KismetSystemLibrary.PrintString` "Hello")
                (set `self.FrontDoDamage?` false)
                (`/Game/GAME/BP/BP_Player.TakeDamage` (`self.As BP Player`) (`/Game/GAME/BP/Components/BPC_Damagable.Damage` (`self.BPC_Damagable`)))))))))))

(event `Attack2`
  (bind _fronthitbox (`self.FrontHitBox`))
  (set `self.Can Attack` false)
  (set `self.Is Second Attacking` true)
  (`KismetSystemLibrary.Delay` 0.6)
  (set `self.FrontDoDamage?` true)
  (`GameplayStatics.PlaySound2D` "/Game/GAME/SOUND/SOUNDEFFECT/Splash_Sound_Effect.Splash_Sound_Effect" 1.0 1.0 0.0 null null)
  (`SceneComponent.SetVisibility` _fronthitbox true false)
  (`KismetSystemLibrary.Delay` 0.2)
  (`SceneComponent.SetVisibility` _fronthitbox false false)
  (set `self.FrontDoDamage?` false)
  (`KismetSystemLibrary.Delay` 0.1)
  (set `self.Is Second Attacking` false)
  (set `self.Follow Player` true)
  (`self.Cooldown Attack`))

(event `Attack1`
  (bind _tailhitbox (`self.TailHitBox`))
  (set `self.Can Attack` false)
  (set `self.Is First Attacking` true)
  (`KismetSystemLibrary.Delay` 0.5)
  (set `self.TailDoDamage?` true)
  (`SceneComponent.SetVisibility` _tailhitbox true false)
  (`KismetSystemLibrary.Delay` 0.6)
  (`SceneComponent.SetVisibility` _tailhitbox false false)
  (set `self.TailDoDamage?` false)
  (`KismetSystemLibrary.Delay` 0.2)
  (set `self.Is First Attacking` false)
  (set `self.Follow Player` true)
  (`self.Cooldown Attack`))

(event `Cooldown Attack`
  (if (not (`self.Can Attack`))
    (`KismetSystemLibrary.Delay` 2.5)
    (set `self.Can Attack` true)))

(event `ChooseAttack`
  (if (`self.Can Attack`)
    (set `self.Follow Player` false)
    (if (`KismetMathLibrary.RandomBool`)
      (`self.Attack1`)
      (else
        (`self.Attack2`)))))

(fn `UserConstructionScript`)