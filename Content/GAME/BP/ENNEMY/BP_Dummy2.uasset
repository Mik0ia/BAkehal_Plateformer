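; BP_Dummy2 is a training dummy enemy that takes damage equal to the player's level, showing it briefly in a damage widget.
; Hits subtract from BPCEnnemy's HP, with a TakingDamage flag and short delays blocking repeat hits.
; The first dummy also shows an input prompt once the GameInstance signals the sword unlock, hiding it during hits.
; On death it adds score, tips the mesh over via timeline, then removes its collision and damage box.
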(event `self.ReceiveBeginPlay`
  (bind _aswbp_take_damage (cast `/Game/GAME/BP/WBP/WBP_Take_Damage` (`WidgetComponent.GetWidget` (`self.Damage`))))
  (set `self.As WBP Take Damage` _aswbp_take_damage)
  (bind _aswbp_input (cast `/Game/GAME/BP/WBP/WBP_Input` (`WidgetComponent.GetWidget` (`self.Input`))))
  (set `/Game/GAME/BP/WBP/WBP_Input.ImageIndex` 2 _aswbp_input)
  (if (`self.IsFirstDummy?`)
    (bind _asbp_game_instance (cast `/Game/GAME/BP/BP_GameInstance` (`GameplayStatics.GetGameInstance`)))
    (add `/Game/GAME/BP/BP_GameInstance.SwordUnlocked` _asbp_game_instance (delegate `InputVisible`))))

(event `InputVisible`
  (`SceneComponent.SetVisibility` (`self.Input`) true false))

(event `/Game/GAME/BP/BPI/BPI_EnnemyDamagable.Take_damage`
  (params (Player_Level :type Integer))
  (bind _bpc_ennemy (`self.BPC_Ennemy`))
  (bind _skeletalmesh (`self.SkeletalMesh`))
  (bind _returnvalue (`SceneComponent.GetRelativeTransform` _skeletalmesh))
  (bind _returnvalue_2 (- (`/Game/GAME/BP/Components/BPC_Ennemy.Hp` _bpc_ennemy) Player_Level))
  (if (not (`self.Taking Damage`))
    (set `self.Taking Damage` true)
    (if (`self.IsFirstDummy?`)
      (`SceneComponent.SetVisibility` (`self.Input`) false false))
    (`/Game/GAME/BP/WBP/WBP_Take_Damage.take_damage` (`self.As WBP Take Damage`) Player_Level)
    (`SceneComponent.SetVisibility` (`self.Damage`) true false)
    (if (<= _returnvalue_2 0)
      (`|ExecutionSequence`
        (:`then_0`
          (if (`self.IsFirstDummy?`)
            (`SceneComponent.SetVisibility` (`self.Input`) false false))
          (bind _asbp_game_instance (cast `/Game/GAME/BP/BP_GameInstance` (`GameplayStatics.GetGameInstance`)))
          (`/Game/GAME/BP/BP_GameInstance.IncreaseScore` _asbp_game_instance 3 0)
          (`KismetSystemLibrary.Delay` 0.2)
          (`SceneComponent.SetVisibility` (`self.Damage`) false false))
        (:`then_1`
          (bind (_direction _die) (`Timeline|Dying` :!via `PlayFromStart`)
            (:`Update`
              (`SceneComponent.K2_SetRelativeRotation` _skeletalmesh (`KismetMathLibrary.MakeRotator` (.roll (.rotation _returnvalue)) _die (.yaw (.rotation _returnvalue))) false false))
            (:`Finished`
              (`ActorComponent.K2_DestroyComponent` (`self.Collision`))
              (`ActorComponent.K2_DestroyComponent` (`self.DamageBox`))))))
      (else
        (set `/Game/GAME/BP/Components/BPC_Ennemy.Hp` _returnvalue_2 _bpc_ennemy)
        (`KismetSystemLibrary.Delay` 0.2)
        (`SceneComponent.SetVisibility` (`self.Damage`) false false)
        (`KismetSystemLibrary.Delay` 0.4)
        (if (`self.IsFirstDummy?`)
          (`SceneComponent.SetVisibility` (`self.Input`) true false))
        (set `self.Taking Damage` false)))))

(fn `UserConstructionScript`)