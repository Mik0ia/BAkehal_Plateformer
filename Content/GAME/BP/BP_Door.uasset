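; BP_Door is an interactable door that opens only once the game instance's SwitchValues reaches 3.
; Activating its BPC_Interactable component then plays a success sound and a timeline that rotates the mesh's yaw.
; Otherwise, activation toggles a WBP_TalkingBox widget showing the text line indexed by the current SwitchValues.
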(event `self.ReceiveBeginPlay`
  (bind _asbp_game_instance (cast `/Game/GAME/BP/BP_GameInstance` (`GameplayStatics.GetGameInstance`)))
  (set `self.As BP Game Instance` _asbp_game_instance)
  (bind _aswbp_talking_box (cast `/Game/GAME/BP/WBP/WBP_TalkingBox` (`WidgetComponent.GetWidget` (`self.Widget`))))
  (set `self.As WBP Talking Box` _aswbp_talking_box))

(event `self.BPC_Interactable.OnComponentActivated`
  (params (Component :type "ActorComponent Object Reference") (bReset :type Boolean))
  (bind _switchvalues (`/Game/GAME/BP/BP_GameInstance.SwitchValues` (`self.As BP Game Instance`)))
  (if (`self.IsInteracting?`)
    (set `self.IsInteracting?` false)
    (`SceneComponent.SetVisibility` (`self.Widget`) false false)
    (elif (== _switchvalues 3)
      (`GameplayStatics.PlaySound2D` "/Game/GAME/SOUND/SOUNDEFFECT/Success_Sound_Effect.Success_Sound_Effect" 0.5 1.0 0.2 null null)
      (bind (_direction _rotate) (`Timeline|Timeline`)
        (:`Update`
          (`SceneComponent.K2_SetRelativeRotation` (`self.StaticMesh`) (`KismetMathLibrary.MakeRotator` 0.0 0.0 (* _rotate -1.0)) false false)))
      (else
        (set `self.IsInteracting?` true)
        (`SceneComponent.SetVisibility` (`self.Widget`) true false)
        (`/Game/GAME/BP/WBP/WBP_TalkingBox.Text` (`self.As WBP Talking Box`) (`|GetArrayItem` (`self.Text`) _switchvalues))))))

(fn `UserConstructionScript`)