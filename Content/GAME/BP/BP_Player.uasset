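; Player character Blueprint handling movement, jumps, swimming, sword attacks, interaction, collectibles, pause menu and death with level reload.
; BP_GameInstance holds HP and sword/double-jump unlocks, pushing unlock and score events to player and HUD.
; Tick glides the camera along the nearest spline unless CamBoss is set, and polls the sword hitbox.
; Components identify collectibles, interactables, damageables and depth-movement zones; pausing slows time dilation, with move/jump inputs driving the menu.
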(event `EnhancedInput|/Game/GAME/INPUT/Actions/IA_Pause`
  (params (ActionValue :type Boolean) (ElapsedSeconds :type "Float (double-precision)") (TriggeredSeconds :type "Float (double-precision)") (InputAction :type "InputAction Object Reference" :default "/Game/GAME/INPUT/Actions/IA_Pause.IA_Pause"))
  ;[0.3625 1 0.3474] Activer et désactiver le menu pause
  (:`Started`
    (`GameplayStatics.PlaySound2D` "/Game/GAME/SOUND/SOUNDEFFECT/Best_Pause_Sound_Effect.Best_Pause_Sound_Effect" 2.5 1.0 0.2 null null)
    (if (`self.IsInPauseMenu?`)
      (`GameplayStatics.SetGlobalTimeDilation` 1.0)
      (`Widget.RemoveFromParent` (`self.PauseMenuRef`))
      (set `self.IsInPauseMenu?` false)
      (else
        (`GameplayStatics.SetGlobalTimeDilation` 0.2)
        (bind _returnvalue (`|CreateWidget` "/Game/GAME/BP/WBP/WBP_PauseMenu.WBP_PauseMenu_C"))
        (bind _output_get (set `self.PauseMenuRef` _returnvalue))
        (`UserWidget.AddToViewport` _output_get 0)
        (set `self.IsInPauseMenu?` true)))))

(event `self.ReceiveBeginPlay`
  (bind _returnvalue (`self.K2_GetActorLocation`))
  (bind _bpc_player (`self.BPC_Player`))
  (`parent.ReceiveBeginPlay`)
  (bind _returnvalue_2 (`|CreateWidget` "/Game/GAME/BP/WBP/WBP_MainHud.WBP_MainHud_C"))
  (bind _output_get (set `self.Widget` _returnvalue_2))
  (`UserWidget.AddToViewport` _output_get 0)
  (`/Game/GAME/BP/WBP/WBP_MainHud.update score` _output_get)
  (bind _returnvalue_3 (`GameplayStatics.GetActorOfClass` "/Game/GAME/BP/Manager/BP_SplineManager.BP_SplineManager_C"))
  (bind _output_get_2 (set `self.Bp Splines Ref` (`/Game/GAME/BP/Manager/BP_SplineManager.Bp_Splines_Ref` _returnvalue_3)))
  (bind _output (`|GetArrayItem` _output_get_2))
  (set `self.ClosestCAM_Ref` _output)
  (set `self.Cam_Min_Lenght` (`KismetMathLibrary.Vector_Distance` (`SplineComponent.FindLocationClosestToWorldLocation` (`/Game/GAME/BP/Manager/BP_SplineCAM.Spline` _output) _returnvalue "World") _returnvalue))
  (bind _asbp_game_instance (cast `/Game/GAME/BP/BP_GameInstance` (`GameplayStatics.GetGameInstance`)))
  (bind _output_get_3 (set `self.As BP Game Instance` _asbp_game_instance))
  (set `/Game/GAME/BP/BP_GameInstance.As BP Player` self _output_get_3)
  (set `self.JumpMaxCount` (`/Game/GAME/BP/BP_GameInstance.MaxJumpCount` _output_get_3))
  (set `self.SwordUnlocked?` (`/Game/GAME/BP/BP_GameInstance.HasSwordUnlocked` _output_get_3))
  (add `/Game/GAME/BP/BP_GameInstance.SwordUnlocked` _output_get_3 (delegate `SwordUnlocked`))
  (add `/Game/GAME/BP/BP_GameInstance.HasUnlockDBLJump` _output_get_3 (delegate `UnlockDBLJump`))
  (add `/Game/GAME/BP/BP_GameInstance.UpdateScore` _output_get_3 (delegate `UpdateScore`))
  (bind _aswbp_score_player (cast `/Game/GAME/BP/WBP/WBP_ScorePlayer` (`WidgetComponent.GetWidget` (`self.Score`))))
  (set `self.As WBP Score Player` _aswbp_score_player)
  (add `/Game/GAME/BP/Components/BPC_Player.set Is Swimming` _bpc_player (delegate `Swims`))
  (add `/Game/GAME/BP/Components/BPC_Player.Set Isn't Swimming` _bpc_player (delegate `Remove Smimming`))
  (set `self.CamInitialRotation` (`SceneComponent.K2_GetComponentRotation` (`self.FollowCamera`)))
  (bind _outactors (`GameplayStatics.GetAllActorsOfClass` "/Game/GAME/BP/BP_PROPS/Bp_BigDoor.Bp_BigDoor_C"))
  (bind _output_2 (`|GetArrayItem` _outactors))
  (`/Engine/EditorBlueprintResources/StandardMacros.IsValid` _output_2
    (:`Is Valid`
      (add `/Game/GAME/BP/BP_PROPS/Bp_BigDoor.BigDoorOpens` _output_2 (delegate `BigDoorOpens`)))
    (:`Is Not Valid`
      _))
  (if (`self.SwordUnlocked?`)
    (`SceneComponent.SetVisibility` (`self.StaticMesh`) true false)
    (else
      (`SceneComponent.SetVisibility` (`self.StaticMesh`) false false))))

(event `EnhancedInput|/Game/GAME/INPUT/Actions/IA_Move`
  (params (ActionValue :type "Vector2D Structure") (ElapsedSeconds :type "Float (double-precision)") (TriggeredSeconds :type "Float (double-precision)") (InputAction :type "InputAction Object Reference" :default "/Game/GAME/INPUT/Actions/IA_Move.IA_Move"))
  ;[1 1 1] Mouvement du joueur
  (:`Triggered`
    (if (not (`self.IsInPauseMenu?`))
      (`self.AddMovementInput` (`KismetMathLibrary.GetRightVector` (`KismetMathLibrary.MakeRotator` 0.0)) ActionValue_X)
      (if (`PhysicsVolume.bWaterVolume` (`MovementComponent.GetPhysicsVolume` (`self.CharacterMovement`)))
        (`self.AddMovementInput` (`KismetMathLibrary.GetUpVector` (`KismetMathLibrary.MakeRotator` 0.0)) ActionValue_Y)
        (elif (`/Game/GAME/BP/Components/BPC_Player.CanMoveUpward` (`self.BPC_Player`))
          (`self.AddMovementInput` (`KismetMathLibrary.GetForwardVector` (`KismetMathLibrary.MakeRotator` 0.0)) ActionValue_Y)))
      (elif (`self.MenuJoystickCooldown`)
        _
        (elif (> ActionValue_Y 20.0)
          (set `self.MenuJoystickCooldown` true)
          (`/Game/GAME/BP/WBP/WBP_PauseMenu.ChangeIndex` (`self.PauseMenuRef`) true)
          (elif (< ActionValue_Y -20.0)
            (set `self.MenuJoystickCooldown` true)
            (`/Game/GAME/BP/WBP/WBP_PauseMenu.ChangeIndex` (`self.PauseMenuRef`) false))))))
  (:`Completed`
    ;[0.6663 0.575 1] réactiver le mouvement quand on lache le joystick
    (if (`self.IsInPauseMenu?`)
      (set `self.MenuJoystickCooldown` false))))

(event `Remove Smimming`
  (set `PhysicsVolume.bWaterVolume` false (`MovementComponent.GetPhysicsVolume` (`self.CharacterMovement`))))

(event `SwordUnlocked`
  (set `self.SwordUnlocked?` true)
  (`SceneComponent.SetVisibility` (`self.StaticMesh`) true false))

(event `UpdateScore`
  (`/Game/GAME/BP/WBP/WBP_MainHud.update score` (`self.Widget`)))

(event `Swims`
  (set `PhysicsVolume.bWaterVolume` true (`MovementComponent.GetPhysicsVolume` (`self.CharacterMovement`))))

(event `UnlockDBLJump`
  (set `self.JumpMaxCount` 2))

(event `BigDoorOpens`
  (bind _asplayer_controller (cast `PlayerController` (`self.GetController`)))
  (bind _returnvalue (pcsubsystem `EnhancedInputLocalPlayerSubsystem` _asplayer_controller))
  (`EnhancedInputSubsystemInterface.RemoveMappingContext` _returnvalue "/Game/GAME/INPUT/IMC_Default.IMC_Default" (struct))
  (`GameplayStatics.PlayWorldCameraShake` "/Game/GAME/BP/CAM/Bp_ShakeCameraDoor.Bp_ShakeCameraDoor_C" (`SceneComponent.K2_GetComponentLocation` (`self.FollowCamera`)) 0.0 500.0)
  (`PlayerController.K2_ClientPlayForceFeedback` _asplayer_controller "/Game/GAME/INPUT/FF_DoorOpens.FF_DoorOpens" "None" false false false)
  (bind _returnvalue_2 (`AddComponent|NODE_AddAudioComponent-2`))
  (`AudioComponent.FadeIn` _returnvalue_2 0.0 4.0 0.5 "Linear")
  (`KismetSystemLibrary.Delay` 4.9)
  (`GameplayStatics.PlaySound2D` "/Game/GAME/SOUND/SOUNDEFFECT/rock_wall_smash_sound_effect_fixed_.rock_wall_smash_sound_effect_fixed_" 0.7 1.0 0.2 null null)
  (`AudioComponent.FadeOut` _returnvalue_2 0.0 0.0 "Linear")
  (`KismetSystemLibrary.Delay` 0.1)
  (`EnhancedInputSubsystemInterface.AddMappingContext` _returnvalue "/Game/GAME/INPUT/IMC_Default.IMC_Default" 0 (struct)))

(event `self.ReceiveTick`
  (params (DeltaSeconds :type "Float (single-precision)"))
  (bind _returnvalue (- (`self.K2_GetActorLocation`) (500.0 0.0 0.0)))
  (bind (_camera_angle_x _camera_angle_y _camera_angle_z) (`KismetMathLibrary.BreakVector` (`/Game/GAME/BP/Manager/BP_SplineCAM.Camera Angle` (`self.ClosestCAM_Ref`))))
  (if (not (`self.Is Dead`))
    (`|ExecutionSequence`
      (:`then_0`
        (if (not (`self.Cam Boss ?`))
          ;[1 1 1] Move Camera Along Spline
          (`SceneComponent.K2_SetWorldLocation` (`self.FollowCamera`) (`KismetMathLibrary.VInterpTo` (`SceneComponent.K2_GetComponentLocation` (`self.FollowCamera`)) (`SplineComponent.FindLocationClosestToWorldLocation` (`/Game/GAME/BP/Manager/BP_SplineCAM.Spline` (`self.ClosestCAM_Ref`)) (- (`self.K2_GetActorLocation`) (500.0 0.0 0.0)) "World") (`GameplayStatics.GetWorldDeltaSeconds`) 7.0) false false)
          (`SceneComponent.K2_SetRelativeRotation` (`self.FollowCamera`) (`KismetMathLibrary.MakeRotator` _camera_angle_x _camera_angle_y _camera_angle_z) false false)))
      (:`then_1`
        (if (not (`self.Cam Boss ?`))
          (set `self.Cam_Min_Lenght` 500000.0)
          ;[1 0.3594 0.3594] Code pour choisir le spline cam le plus proche
          (for _array_element (`self.Bp Splines Ref`)
            (bind _returnvalue_2 (`KismetMathLibrary.Vector_Distance` (`SplineComponent.FindLocationClosestToWorldLocation` (`/Game/GAME/BP/Manager/BP_SplineCAM.Spline` _array_element) _returnvalue "World") _returnvalue))
            (if (< _returnvalue_2 (`self.Cam_Min_Lenght`))
              (set `self.Cam_Min_Lenght` _returnvalue_2)
              (set `self.ClosestCAM_Ref` _array_element)))))
      (:`then_2`
        ;[1 0.516 0.4662] mécanique de cancel des attaques si on touche le sol ou on saute
        (if (`NavMovementComponent.IsMovingOnGround` (`self.CharacterMovement`))
          (if (`self.AerialAttacking`)
            (set `self.AerialAttacking` false))
          (elif (`self.is Ground attacking`)
            (set `self.is Ground attacking` false)
            (set `self.cooldown` false))))
      (:`then_3`
        (if (`PhysicsVolume.bWaterVolume` (`MovementComponent.GetPhysicsVolume` (`self.CharacterMovement`)))
          (`/Engine/EditorBlueprintResources/StandardMacros.DoOnce` false :!label _label
            (:`Completed`
              (bind _returnvalue_3 (`AddComponent|NODE_AddAudioComponent-0`))
              (`AudioComponent.FadeIn` _returnvalue_3 0.0 2.0 0.0 "Linear")
              (`KismetSystemLibrary.Delay` 15.0)
              (goto _label :!via `Reset`)))
          (else
            (`/Engine/EditorBlueprintResources/StandardMacros.IsValid` _returnvalue_3
              (:`Is Valid`
                (`AudioComponent.FadeOut` _returnvalue_3 0.0 0.0 "Linear"))))))
      (:`then_4`
        (`self.Attack`)))))

(event `self.ReceiveActorEndOverlap`
  (params (OtherActor :type "Actor Object Reference"))
  ;[1 1 1] supprime les acteurs qui n'overlap plus de l'array
  (`/Engine/EditorBlueprintResources/StandardMacros.IsValid` OtherActor
    (:`Is Valid`
      (if (and (`KismetSystemLibrary.IsValid` (`self.GetComponentByClass` OtherActor "/Game/GAME/BP/Components/BPC_MoveUpwardBox.BPC_MoveUpwardBox_C")) (not (`self.IsOverlappingActor` OtherActor)))
        (set `/Game/GAME/BP/Components/BPC_Player.CanMoveUpward` false (`self.BPC_Player`))))))

(event `ScoreWidget`
  (params (ScoreIndex :type Integer) (Value :type Integer))
  (bind _as_wbp_score_player (`self.As WBP Score Player`))
  ;[1 1 1] Widget qui affiche le score qui augmente
  (switch `int` ScoreIndex
    (:`0`
      (`/Game/GAME/BP/WBP/WBP_ScorePlayer.ScoreIncrease` _as_wbp_score_player Value))
    (:`1`
      (`/Game/GAME/BP/WBP/WBP_ScorePlayer.ScoreIncrease` _as_wbp_score_player Value))
    (:`2`
      (`/Game/GAME/BP/WBP/WBP_ScorePlayer.ScoreIncrease` _as_wbp_score_player 3))
    (:`3`
      (`/Game/GAME/BP/WBP/WBP_ScorePlayer.ScoreIncrease` _as_wbp_score_player Value))
    (:`4`
      (`/Game/GAME/BP/WBP/WBP_ScorePlayer.ScoreIncrease` _as_wbp_score_player Value))
    (:`5`
      (`/Game/GAME/BP/WBP/WBP_ScorePlayer.ScoreIncrease` _as_wbp_score_player Value :!label _label_2))
    (:`6`
      (goto _label_2))))

(event `self.OnJumped`
  ;[1 0.6438 0.2568] code pour les animations de saut et double saut
  (`GameplayStatics.PlaySound2D` "/Game/GAME/SOUND/SOUNDEFFECT/Swipe_Swoosh_Transition_Sound_Effect.Swipe_Swoosh_Transition_Sound_Effect" 0.3 (`KismetMathLibrary.RandomFloatInRange` 1.1 1.4) 0.3 null null)
  (switch `int` (`self.JumpCurrentCount`)
    (:`1`
      (set `self.IsFirstJumping` true)
      (`KismetSystemLibrary.Delay` 0.1)
      (set `self.IsFirstJumping` false))
    (:`2`
      (set `self.IsSecondJumping` true)
      (`KismetSystemLibrary.Delay` 0.3)
      (set `self.IsSecondJumping` false))))

(event `self.ReceiveActorBeginOverlap`
  (params (OtherActor :type "Actor Object Reference"))
  (bind _returnvalue (`self.GetComponentByClass` OtherActor "/Game/GAME/BP/Components/BPC_Collectible_Component.BPC_Collectible_Component_C"))
  ;[0.8439 1 0.3046] Code pour collecter les collectible et permettre au joueur d'allé en profondeur quand il est dans une box qui lui permet
  (`/Engine/EditorBlueprintResources/StandardMacros.IsValid` _returnvalue
    (:`Is Valid`
      (`/Game/GAME/BP/Components/BPC_CollectComponent.Collect` (`self.BPC_CollectComponent`) _returnvalue (`/Game/GAME/BP/Components/BPC_Collectible_Component.Value` _returnvalue) (`/Game/GAME/BP/Components/BPC_Collectible_Component.Index` _returnvalue)))
    (:`Is Not Valid`
      (`/Engine/EditorBlueprintResources/StandardMacros.IsValid` (`self.GetComponentByClass` OtherActor "/Game/GAME/BP/Components/BPC_MoveUpwardBox.BPC_MoveUpwardBox_C")
        (:`Is Valid`
          (set `/Game/GAME/BP/Components/BPC_Player.CanMoveUpward` true (`self.BPC_Player`)))))))

(event `EnhancedInput|/Game/GAME/INPUT/Actions/IA_Attack`
  (params (ActionValue :type Boolean) (ElapsedSeconds :type "Float (double-precision)") (TriggeredSeconds :type "Float (double-precision)") (InputAction :type "InputAction Object Reference" :default "/Game/GAME/INPUT/Actions/IA_Attack.IA_Attack"))
  ;[1 0.06387 0] code pour attacquer qui pernd un booléen correspondant à s'il attauqe au sol ou en l'air, le cooldown dépend de l'animation.
  (:`Started`
    (if (`self.SwordUnlocked?`)
      (if (not (`self.cooldown`))
        (if (not (`PhysicsVolume.bWaterVolume` (`MovementComponent.GetPhysicsVolume` (`self.CharacterMovement`))))
          (`GameplayStatics.PlaySound2D` "/Game/GAME/SOUND/SOUNDEFFECT/Swipe_Swoosh_Transition_Sound_Effect.Swipe_Swoosh_Transition_Sound_Effect" 1.0 2.0 0.3 null null)
          (if (`NavMovementComponent.IsMovingOnGround` (`self.CharacterMovement`))
            (set `self.is Ground attacking` true)
            (set `self.cooldown` true)
            (`KismetSystemLibrary.Delay` 0.65)
            (set `self.is Ground attacking` false)
            (`KismetSystemLibrary.Delay` 0.3)
            (set `self.cooldown` false)
            (else
              (set `self.AerialAttacking` true)
              (set `self.cooldown` true)
              (`KismetSystemLibrary.Delay` 1.0)
              (set `self.AerialAttacking` false)
              (set `self.cooldown` false))))))))

(event `EnhancedInput|/Game/GAME/INPUT/Actions/IA_debug`
  (params (ActionValue :type Boolean) (ElapsedSeconds :type "Float (double-precision)") (TriggeredSeconds :type "Float (double-precision)") (InputAction :type "InputAction Object Reference" :default "/Game/GAME/INPUT/Actions/IA_debug.IA_debug"))
  (bind _as_bp_game_instance (`self.As BP Game Instance`))
  ;[1 0 0.9862] debug
  (:`Started`
    (`/Game/GAME/BP/BP_GameInstance.Unlock Sword` _as_bp_game_instance)
    (`/Game/GAME/BP/BP_GameInstance.UnlockDBLJump` _as_bp_game_instance)
    (set `/Game/GAME/BP/BP_GameInstance.HasBambooPerdu` true _as_bp_game_instance)
    (set `/Game/GAME/BP/BP_GameInstance.HasFirstCrystal?` true _as_bp_game_instance)
    (set `/Game/GAME/BP/BP_GameInstance.HasSecondCrystal?` true _as_bp_game_instance)))

(event `self.Sphere.OnComponentBeginOverlap`
  (params (OverlappedComponent :type "PrimitiveComponent Object Reference") (OtherActor :type "Actor Object Reference") (OtherComp :type "PrimitiveComponent Object Reference") (OtherBodyIndex :type Integer) (bFromSweep :type Boolean) (SweepResult :type "HitResult Structure (by ref)"))
  ;[1 0.1927 0.1927] Stockage des Acteur qui peuevnt intéragir
  ;;[1 1 1] stock les acteurs qui peuvent intéragir dans un array
  (`/Engine/EditorBlueprintResources/StandardMacros.IsValid` (`self.GetComponentByClass` OtherActor "/Game/GAME/BP/Components/BPC_Interactable.BPC_Interactable_C")
    (:`Is Valid`
      (`KismetArrayLibrary.Array_Add` (`self.InteractableActor`) OtherActor))))

(event `self.Sphere.OnComponentEndOverlap`
  (params (OverlappedComponent :type "PrimitiveComponent Object Reference") (OtherActor :type "Actor Object Reference") (OtherComp :type "PrimitiveComponent Object Reference") (OtherBodyIndex :type Integer))
  ;[1 0.1927 0.1927] Stockage des Acteur qui peuevnt intéragir
  ;;[1 1 1] Enlève les Acteurs qui peuvent intéragir de l'Array
  (`/Engine/EditorBlueprintResources/StandardMacros.IsValid` (`self.GetComponentByClass` OtherActor "/Game/GAME/BP/Components/BPC_Interactable.BPC_Interactable_C")
    (:`Is Valid`
      (`KismetArrayLibrary.Array_RemoveItem` (`self.InteractableActor`) OtherActor))))

(event `EnhancedInput|/Game/GAME/INPUT/Actions/IA_Interact`
  (params (ActionValue :type Boolean) (ElapsedSeconds :type "Float (double-precision)") (TriggeredSeconds :type "Float (double-precision)") (InputAction :type "InputAction Object Reference" :default "/Game/GAME/INPUT/Actions/IA_Interact.IA_Interact"))
  (bind _output (`|GetArrayItem` (`self.InteractableActor`)))
  ;[1 0.2812 0.2812] Intéragir avec le premier acteur stocker
  (:`Started`
    (`/Engine/EditorBlueprintResources/StandardMacros.IsValid` _output
      (:`Is Valid`
        (`ActorComponent.Activate` (`self.GetComponentByClass` _output "/Game/GAME/BP/Components/BPC_Interactable.BPC_Interactable_C") true)))))

(event `EnhancedInput|/Game/GAME/INPUT/Actions/IA_Jump`
  (params (ActionValue :type Boolean) (ElapsedSeconds :type "Float (double-precision)") (TriggeredSeconds :type "Float (double-precision)") (InputAction :type "InputAction Object Reference" :default "/Game/GAME/INPUT/Actions/IA_Jump.IA_Jump"))
  (bind _pausemenuref (`self.PauseMenuRef`))
  (:`Started`
    (if (`self.IsInPauseMenu?`)
      (`GameplayStatics.PlaySound2D` "/Game/GAME/SOUND/SOUNDEFFECT/Confirm_Button_Sound_Effect.Confirm_Button_Sound_Effect" 4.0 1.0 0.2 null null)
      (switch `int` (`/Game/GAME/BP/WBP/WBP_PauseMenu.Index` _pausemenuref)
        (:`0`
          (`Widget.RemoveFromParent` _pausemenuref)
          (set `self.IsInPauseMenu?` false)
          (`GameplayStatics.SetGlobalTimeDilation` 1.0))
        (:`1`
          (`GameplayStatics.OpenLevelBySoftObjectPtr` "/Game/GAME/MAP/MainMenu.MainMenu"))
        (:`2`
          (`KismetSystemLibrary.QuitGame` null "Quit")))
      (else
        (`self.Jump`))))
  (:`Completed`
    (`self.StopJumping`)))

(event `Attack`
  (bind _actoralreadyattacked (`self.ActorAlreadyAttacked`))
  (if (or (`self.is Ground attacking`) (`self.AerialAttacking`))
    (for _array_element (`PrimitiveComponent.GetOverlappingActors` (`self.Hitbox Sword`) null)
      (bind _returnvalue (`self.GetComponentByClass` _array_element "/Game/GAME/BP/Components/BPC_Damagable.BPC_Damagable_C"))
      (`/Engine/EditorBlueprintResources/StandardMacros.IsValid` _returnvalue
        (:`Is Valid`
          (if (not (`KismetArrayLibrary.Array_Contains` _actoralreadyattacked (stale _array_element_2)))
            (`KismetArrayLibrary.Array_Add` _actoralreadyattacked _returnvalue)
            (for _array_element_2 _actoralreadyattacked
              (`/Game/GAME/BP/Components/BPC_Damagable.Takedamage` _returnvalue))))))
    (else
      (`KismetArrayLibrary.Array_Clear` (`self.ActorAlreadyAttacked`)))))

(event `TakeDamage`
  (params (`Ennemy Damage` :type Integer))
  (bind _as_bp_game_instance (`self.As BP Game Instance`))
  (bind _as_bp_game_instance_2 (`self.As BP Game Instance`))
  (bind _returnvalue (- (`/Game/GAME/BP/BP_GameInstance.PlayerHP` _as_bp_game_instance) `Ennemy Damage`))
  (`PlayerController.K2_ClientPlayForceFeedback` (`GameplayStatics.GetPlayerController` 0) "/Game/GAME/INPUT/FF_Hit.FF_Hit" "None" false false false)
  (`/Engine/EditorBlueprintResources/StandardMacros.IsValid` (stale _returnvalue_2)
    (:`Is Valid`
      (`Widget.RemoveFromParent` (stale _returnvalue_2)))
    (:`Is Not Valid`
      _))
  (bind _returnvalue_2 (`|CreateWidget` "/Game/GAME/BP/WBP/WBP_Damage.WBP_Damage_C"))
  (`UserWidget.AddToViewport` _returnvalue_2 0)
  (if (> _returnvalue 0)
    (set `/Game/GAME/BP/BP_GameInstance.PlayerHP` _returnvalue _as_bp_game_instance)
    (`self.UpdateScore`)
    (`GameplayStatics.PlaySound2D` "/Game/GAME/SOUND/SOUNDEFFECT/Cue/Hit_Kenshin1.Hit_Kenshin1" 1.0 (`KismetMathLibrary.RandomFloatInRange` 0.97 1.03) 0.0 null null)
    (`GameplayStatics.PlayWorldCameraShake` "/Game/GAME/BP/CAM/Bp_ShakeDamage.Bp_ShakeDamage_C" (`SceneComponent.K2_GetComponentLocation` (`self.FollowCamera`)) 0.0 500.0)
    (else
      (set `self.Is Dead` true)
      (set `/Game/GAME/BP/BP_GameInstance.PlayerHP` 0 _as_bp_game_instance)
      (`GameplayStatics.PlaySound2D` "/Game/GAME/SOUND/SOUNDEFFECT/Cue/Death_Kenshin.Death_Kenshin" 1.0 (`KismetMathLibrary.RandomFloatInRange` 0.97 1.03) 0.0 null null)
      (bind _asplayer_controller (cast `PlayerController` (`self.GetController`)))
      (`EnhancedInputSubsystemInterface.RemoveMappingContext` (pcsubsystem `EnhancedInputLocalPlayerSubsystem` _asplayer_controller) "/Game/GAME/INPUT/IMC_Default.IMC_Default" (struct))
      (`self.UpdateScore`)
      (bind _returnvalue_3 (`|CreateWidget` "/Game/GAME/BP/WBP/WBP_FadeToBlack.WBP_FadeToBlack_C"))
      (`UserWidget.AddToViewport` _returnvalue_3 0)
      (`/Game/GAME/BP/WBP/WBP_FadeToBlack.Die` _returnvalue_3)
      (`KismetSystemLibrary.Delay` 1.5)
      (bind _returnvalue_4 (`GameplayStatics.GetCurrentLevelName` true))
      (`GameplayStatics.OpenLevel` (`KismetStringLibrary.Conv_StringToName` _returnvalue_4))
      (set `/Game/GAME/BP/BP_GameInstance.PlayerHP` (`/Game/GAME/BP/BP_GameInstance.MaxPlayerHp` _as_bp_game_instance_2) _as_bp_game_instance_2))))

(event `EnhancedInput|/Game/GAME/INPUT/Actions/IA_debug`
  (params (ActionValue :type Boolean) (ElapsedSeconds :type "Float (double-precision)") (TriggeredSeconds :type "Float (double-precision)") (InputAction :type "InputAction Object Reference" :default "/Game/GAME/INPUT/Actions/IA_debug.IA_debug"))
  (:`Started`
    (bind _asbp_game_instance (cast `/Game/GAME/BP/BP_GameInstance` (`GameplayStatics.GetGameInstance`)))
    (set `/Game/GAME/BP/BP_GameInstance.MaxJumpCount` 2 _asbp_game_instance)
    (set `/Game/GAME/BP/BP_GameInstance.HasSwordUnlocked` true _asbp_game_instance)))

(fn `UserConstructionScript`
  (`parent.UserConstructionScript`))