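; BP_Dummy2 is a damage dummy that displays feedback when it takes a hit.
; Its TakeDamage event passes the PlayerLevel value to the WBP_Take_Damage widget on its Widget component and makes that component visible.
; A TakingDamage flag ignores further hits during a short delay, after which the widget is hidden and the flag clears.
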(event `self.ReceiveTick`
  (params (DeltaSeconds :type "Float (single-precision)")))

(event `/Game/GAME/BP/BPI_EnnemyDamagable.Take_damage`
  (params (Player_Level :type Integer))
  (if (not (`self.Taking Damage`))
    (set `self.Taking Damage` true)
    (bind _aswbp_take_damage (cast `/Game/GAME/BP/WBP_Take_Damage` (`WidgetComponent.GetWidget` (`self.Widget`))))
    (`/Game/GAME/BP/WBP_Take_Damage.take_damage` _aswbp_take_damage Player_Level)
    (`SceneComponent.SetVisibility` (`self.Widget`) true false)
    (`KismetSystemLibrary.Delay` 0.2)
    (set `self.Taking Damage` false)
    (`SceneComponent.SetVisibility` (`self.Widget`) false false)))

(fn `UserConstructionScript`)