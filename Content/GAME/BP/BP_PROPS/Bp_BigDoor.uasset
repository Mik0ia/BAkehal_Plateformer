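; Big double door that opens once both crystals are placed in their sockets, as tracked in the game instance.
; A sphere overlap shows an input prompt to the player, and activating the interactable either opens the door or toggles a talking-box hint about the missing crystals.
; Opening runs two timelines that swing each panel's yaw and saves the open state in the game instance, which BeginPlay reads to restore it.
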(event `self.ReceiveBeginPlay`
  (bind _doorleft (`self.DoorLeft`))
  (bind _doorright (`self.DoorRight`))
  (bind (_returnvalue_roll _returnvalue_pitch) (`KismetMathLibrary.BreakRotator` (`SceneComponent.K2_GetComponentRotation` _doorright)))
  (bind (_returnvalue_roll_2 _returnvalue_pitch_2) (`KismetMathLibrary.BreakRotator` (`SceneComponent.K2_GetComponentRotation` _doorleft)))
  (bind _aswbp_input (cast `/Game/GAME/BP/WBP/WBP_Input` (`WidgetComponent.GetWidget` (`self.Input`))))
  (set `/Game/GAME/BP/WBP/WBP_Input.ImageIndex` 3 _aswbp_input)
  (bind _asbp_game_instance (cast `/Game/GAME/BP/BP_GameInstance` (`GameplayStatics.GetGameInstance`)))
  (set `self.As BP Game Instance` _asbp_game_instance)
  (bind _aswbp_talking_box (cast `/Game/GAME/BP/WBP/WBP_TalkingBox` (`WidgetComponent.GetWidget` (`self.Text`))))
  (set `self.As WBP Talking Box` _aswbp_talking_box)
  (if (`/Game/GAME/BP/BP_GameInstance.BigDoorIsOpen?` (`self.As BP Game Instance`))
    (set `self.Is open?` true)
    (`SceneComponent.K2_SetRelativeRotation` _doorleft (`KismetMathLibrary.MakeRotator` _returnvalue_roll_2 _returnvalue_pitch_2 -90.0) false false)
    (`SceneComponent.K2_SetRelativeRotation` _doorright (`KismetMathLibrary.MakeRotator` _returnvalue_roll _returnvalue_pitch -90.0) false false)))

(event `self.Sphere.OnComponentBeginOverlap`
  (params (OverlappedComponent :type "PrimitiveComponent Object Reference") (OtherActor :type "Actor Object Reference") (OtherComp :type "PrimitiveComponent Object Reference") (OtherBodyIndex :type Integer) (bFromSweep :type Boolean) (SweepResult :type "HitResult Structure (by ref)"))
  (if (not (`self.Is open?`))
    (`/Engine/EditorBlueprintResources/StandardMacros.IsValid` (`self.GetComponentByClass` OtherActor "/Game/GAME/BP/Components/BPC_Player.BPC_Player_C")
      (:`Is Valid`
        (`SceneComponent.SetVisibility` (`self.Input`) true false)))))

(event `self.Sphere.OnComponentEndOverlap`
  (params (OverlappedComponent :type "PrimitiveComponent Object Reference") (OtherActor :type "Actor Object Reference") (OtherComp :type "PrimitiveComponent Object Reference") (OtherBodyIndex :type Integer))
  (if (not (`self.Is open?`))
    (`/Engine/EditorBlueprintResources/StandardMacros.IsValid` (`self.GetComponentByClass` OtherActor "/Game/GAME/BP/Components/BPC_Player.BPC_Player_C")
      (:`Is Valid`
        (`SceneComponent.SetVisibility` (`self.Input`) false false)))))

(event `self.BPC_Interactable.OnComponentActivated`
  (params (Component :type "ActorComponent Object Reference") (bReset :type Boolean))
  (bind _as_bp_game_instance (`self.As BP Game Instance`))
  (if (not (`self.Is open?`))
    (if (`self.Is Talking ?`)
      (set `self.Is Talking ?` false)
      (`SceneComponent.SetVisibility` (`self.Text`) false false)
      (elif (and (`|GetArrayItem` (`/Game/GAME/BP/BP_GameInstance.HasPlacedCrystal1?` _as_bp_game_instance)) (`|GetArrayItem` (`/Game/GAME/BP/BP_GameInstance.HasPlacedCrystal2?` _as_bp_game_instance)))
        (`SceneComponent.SetVisibility` (`self.Input`) false false)
        (`self.Opens`)
        (else
          (`SceneComponent.SetVisibility` (`self.Text`) true false)
          (set `self.Is Talking ?` true)
          (`/Game/GAME/BP/WBP/WBP_TalkingBox.Text` (`self.As WBP Talking Box`) "Pour ouvrir cette porte il faut placer les 2 cristaux dans leurs socles"))))))

(event `Opens`
  (bind _doorleft (`self.DoorLeft`))
  (bind _doorright (`self.DoorRight`))
  (bind (_returnvalue_roll _returnvalue_pitch) (`KismetMathLibrary.BreakRotator` (`SceneComponent.K2_GetComponentRotation` _doorleft)))
  (bind (_returnvalue_roll_2 _returnvalue_pitch_2) (`KismetMathLibrary.BreakRotator` (`SceneComponent.K2_GetComponentRotation` _doorright)))
  (set `/Game/GAME/BP/BP_GameInstance.BigDoorIsOpen?` true (`self.As BP Game Instance`))
  (set `self.Is open?` true)
  (`|ExecutionSequence`
    (:`then_0`
      (bind (_direction _newtrack_0) (`Timeline|Door1` :!via `PlayFromStart`)
        (:`Update`
          (`SceneComponent.K2_SetRelativeRotation` _doorleft (`KismetMathLibrary.MakeRotator` _returnvalue_roll _returnvalue_pitch _newtrack_0) false false))))
    (:`then_1`
      (bind (_direction_2 _newtrack_0_2) (`Timeline|Door2` :!via `PlayFromStart`)
        (:`Update`
          (`SceneComponent.K2_SetRelativeRotation` _doorright (`KismetMathLibrary.MakeRotator` _returnvalue_roll_2 _returnvalue_pitch_2 _newtrack_0_2) false false))))))

(fn `UserConstructionScript`)