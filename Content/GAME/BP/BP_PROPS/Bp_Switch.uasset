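; Bp_Switch is a one-shot switch prop that adds to a shared switch count when activated.
; On BeginPlay it caches a reference to BP_GameInstance.
; When its BPC_Interactable component fires OnComponentActivated, it sets an IsActivated flag and increments SwitchValues on the game instance, ignoring later activations.
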(event `self.ReceiveBeginPlay`
  (bind _asbp_game_instance (cast `/Game/GAME/BP/BP_GameInstance` (`GameplayStatics.GetGameInstance`)))
  (set `self.As BP Game Instance` _asbp_game_instance))

(event `self.BPC_Interactable.OnComponentActivated`
  (params (Component :type "ActorComponent Object Reference") (bReset :type Boolean))
  (bind _as_bp_game_instance (`self.As BP Game Instance`))
  (if (not (`self.IsActivated?`))
    (set `self.IsActivated?` true)
    (set `/Game/GAME/BP/BP_GameInstance.SwitchValues` (+ (`/Game/GAME/BP/BP_GameInstance.SwitchValues` _as_bp_game_instance) 1) _as_bp_game_instance)))

(fn `UserConstructionScript`)