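; Interactable pedestal that receives the two collectible crystals, with each holder identified by its Index.
; On activation it places an owned crystal not yet set, revealing its mesh with a bling sound and blocking a second crystal on the first's holder.
; GameInstance arrays store placed state and holder Index, which BeginPlay reads to restore visibility.
; Without a crystal to place, it toggles a French hint saying Koi Dragons guard the crystals.
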(event `self.ReceiveBeginPlay`
  (bind _aswbp_talking_box (cast `/Game/GAME/BP/WBP/WBP_TalkingBox` (`WidgetComponent.GetWidget` (`self.Widget`))))
  (set `self.As WBP Talking Box` _aswbp_talking_box)
  (bind _asbp_game_instance (cast `/Game/GAME/BP/BP_GameInstance` (`GameplayStatics.GetGameInstance`)))
  (bind _output_get (set `self.As BP Game Instance` _asbp_game_instance))
  (bind _hasplacedcrystal1_ (`/Game/GAME/BP/BP_GameInstance.HasPlacedCrystal1?` _output_get))
  (if (`|GetArrayItem` _hasplacedcrystal1_)
    (if (== (`self.Index`) (`|GetArrayItem` _hasplacedcrystal1_ 1))
      (`SceneComponent.SetVisibility` (`self.Crystal1`) true false)
      (else
        (bind _hasplacedcrystal2_ (`/Game/GAME/BP/BP_GameInstance.HasPlacedCrystal2?` _output_get))
        (if (`|GetArrayItem` _hasplacedcrystal2_) :!label _label
          (if (== (`|GetArrayItem` _hasplacedcrystal2_ 1) (`self.Index`))
            (`SceneComponent.SetVisibility` (`self.Crystal2`) true false)))))
    (else
      (goto _label))))

(event `self.BPC_Interactable.OnComponentActivated`
  (params (Component :type "ActorComponent Object Reference") (bReset :type Boolean))
  (bind _as_bp_game_instance (`self.As BP Game Instance`))
  (bind _as_bp_game_instance_2 (`self.As BP Game Instance`))
  (bind _hasplacedcrystal1_ (`/Game/GAME/BP/BP_GameInstance.HasPlacedCrystal1?` _as_bp_game_instance_2))
  (bind _hasplacedcrystal2_ (`/Game/GAME/BP/BP_GameInstance.HasPlacedCrystal2?` _as_bp_game_instance_2))
  (bind _output (`|GetArrayItem` _hasplacedcrystal1_))
  (if (`self.Is Talking? ?`)
    (`SceneComponent.SetVisibility` (`self.Widget`) false false)
    (set `self.Is Talking? ?` false)
    (elif (!= (and (`|GetArrayItem` (`/Game/GAME/BP/BP_GameInstance.HasPlacedCrystal1?` _as_bp_game_instance)) (`|GetArrayItem` (`/Game/GAME/BP/BP_GameInstance.HasPlacedCrystal2?` _as_bp_game_instance))) true)
      (if (`/Game/GAME/BP/BP_GameInstance.HasFirstCrystal?` _as_bp_game_instance_2)
        (if _output
          (if (`/Game/GAME/BP/BP_GameInstance.HasSecondCrystal?` _as_bp_game_instance_2) :!label _label_2
            (if (and (`|GetArrayItem` _hasplacedcrystal2_) false)
              _
              (elif _output
                (if (not (== (`|GetArrayItem` _hasplacedcrystal1_ 1) (`self.Index`)))
                  (`KismetArrayLibrary.Array_Set` _hasplacedcrystal2_ 0 true :!label _label_3)
                  (`KismetArrayLibrary.Array_Set` _hasplacedcrystal2_ 1 (`self.Index`))
                  (`SceneComponent.SetVisibility` (`self.Crystal2`) true false)
                  (`GameplayStatics.PlaySound2D` "/Game/GAME/SOUND/SOUNDEFFECT/Diamond_Bling_Sound_Effect__No_copyright_sound_effects___Sounds.Diamond_Bling_Sound_Effect__No_copyright_sound_effects___Sounds" 1.0 (`KismetMathLibrary.RandomFloatInRange` 0.95 1.05) 0.2 null null))
                (else
                  (goto _label_3))))
            (else
              (`SceneComponent.SetVisibility` (`self.Widget`) true false)
              (`/Game/GAME/BP/WBP/WBP_TalkingBox.Text` (`self.As WBP Talking Box`) "Les cristaux sont gardés par les Dragons Koi dans chaque niveaux")
              (set `self.Is Talking? ?` true)))
          (else
            (`KismetArrayLibrary.Array_Set` _hasplacedcrystal1_ 0 true)
            (`KismetArrayLibrary.Array_Set` _hasplacedcrystal1_ 1 (`self.Index`))
            (`SceneComponent.SetVisibility` (`self.Crystal1`) true false)
            (`GameplayStatics.PlaySound2D` "/Game/GAME/SOUND/SOUNDEFFECT/Diamond_Bling_Sound_Effect__No_copyright_sound_effects___Sounds.Diamond_Bling_Sound_Effect__No_copyright_sound_effects___Sounds" 1.0 (`KismetMathLibrary.RandomFloatInRange` 0.95 1.05) 0.2 null null)))
        (else
          (goto _label_2))))))

(fn `UserConstructionScript`)