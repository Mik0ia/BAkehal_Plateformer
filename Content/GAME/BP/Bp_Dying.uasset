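; Interactable actor, apparently a dying character, that delivers a short dialogue and then unlocks the player's sword.
; An overlap sphere shows an input prompt, and each activation of its interactable component steps through a text array in a talking-box widget.
; After the last line it hides the text, unlocks the sword on the game instance, and destroys the player blocker and interaction sphere.
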(event `self.ReceiveBeginPlay`
  (bind _aswbp_talking_box (cast `/Game/GAME/BP/WBP_TalkingBox` (`WidgetComponent.GetWidget` (`self.Tetx`))))
  (set `self.As WBP Talking Box` _aswbp_talking_box))

(event `self.BPC_Interactable.OnComponentActivated`
  (params (Component :type "ActorComponent Object Reference") (bReset :type Boolean))
  (bind _asbp_game_instance (cast `/Game/GAME/BP/BP_GameInstance` (`GameplayStatics.GetGameInstance`)))
  (bind _output_get (set `self.As BP Game Instance` _asbp_game_instance))
  (if (`/Game/GAME/BP/BP_GameInstance.HasSwordUnlocked` _output_get)
    _
    (elif (`self.IsInteracting?`)
      (switch `int` (`self.DialogueIndex`)
        (:`1`
          (`self.Talking`))
        (:`2`
          (`self.Talking`))
        (:`3`
          (`self.Talking`))
        (:`4`
          (`SceneComponent.SetVisibility` (`self.Tetx`) false false)
          (`/Game/GAME/BP/BP_GameInstance.Unlock Sword` (`self.As BP Game Instance`))
          (`ActorComponent.K2_DestroyComponent` (`self.BlocPlayer`))
          (`ActorComponent.K2_DestroyComponent` (`self.InteractibelSphere`))))
      (else
        (`SceneComponent.SetVisibility` (`self.Tetx`) true false)
        (`SceneComponent.SetVisibility` (`self.InputWidget`) false false)
        (`self.Talking`)
        (set `self.IsInteracting?` true)))))

(event `self.InteractibelSphere.OnComponentBeginOverlap`
  (params (OverlappedComponent :type "PrimitiveComponent Object Reference") (OtherActor :type "Actor Object Reference") (OtherComp :type "PrimitiveComponent Object Reference") (OtherBodyIndex :type Integer) (bFromSweep :type Boolean) (SweepResult :type "HitResult Structure (by ref)"))
  (if (not (`self.IsInteracting?`))
    (`SceneComponent.SetVisibility` (`self.InputWidget`) true false)
    (bind _aswbp_input (cast `/Game/GAME/BP/WBP_Input` (`WidgetComponent.GetWidget` (`self.InputWidget`))))
    (set `/Game/GAME/BP/WBP_Input.ImageIndex` 3 _aswbp_input)))

(event `self.InteractibelSphere.OnComponentEndOverlap`
  (params (OverlappedComponent :type "PrimitiveComponent Object Reference") (OtherActor :type "Actor Object Reference") (OtherComp :type "PrimitiveComponent Object Reference") (OtherBodyIndex :type Integer))
  (`SceneComponent.SetVisibility` (`self.InputWidget`) false false))

(fn `Talking`
  (bind _dialogueindex (`self.DialogueIndex`))
  (`/Game/GAME/BP/WBP_TalkingBox.Text` (`self.As WBP Talking Box`) (`|GetArrayItem` (`self.TextArray`) _dialogueindex))
  (set `self.DialogueIndex` (+ _dialogueindex 1)))

(fn `UserConstructionScript`)