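; Water zone manager that tracks which water zones the player is in and switches the player's water state.
; It caches the player pawn as BP_Player on BeginPlay and keeps an array of references added by PutintoWater and removed by RemoveFromWater.
; PutintoWater sets the water flag on the movement component's current physics volume, with a splash sound when it was off.
; RemoveFromWater clears the flag only when the array empties, so multiple zones can overlap.
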(event `self.ReceiveBeginPlay`
  (bind _asbp_player (cast `/Game/GAME/BP/BP_Player` (`GameplayStatics.GetPlayerPawn` 0)))
  (set `self.As BP Player` _asbp_player))

(event `Remove From Water`
  (params (Ref :type "/Game/GAME/BP/Manager/BP_WaterZone Object Reference"))
  (bind _waterzone_array (`self.WaterZone Array`))
  (`KismetArrayLibrary.Array_RemoveItem` _waterzone_array Ref)
  (if (`KismetArrayLibrary.Array_IsEmpty` _waterzone_array)
    (set `PhysicsVolume.bWaterVolume` false (`MovementComponent.GetPhysicsVolume` (`Character.CharacterMovement` (`self.As BP Player`))))))

(event `Put into Water`
  (params (Ref :type "/Game/GAME/BP/Manager/BP_WaterZone Object Reference"))
  (bind _returnvalue (`MovementComponent.GetPhysicsVolume` (`Character.CharacterMovement` (`self.As BP Player`))))
  (`KismetArrayLibrary.Array_Add` (`self.WaterZone Array`) Ref)
  (if (not (`PhysicsVolume.bWaterVolume` _returnvalue))
    (`GameplayStatics.PlaySound2D` "/Game/GAME/SOUND/SOUNDEFFECT/Splash_Sound_Effect.Splash_Sound_Effect" 1.0 1.0 0.0 null null)
    (set `PhysicsVolume.bWaterVolume` true _returnvalue)))

(fn `UserConstructionScript`)