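; Main menu controller Blueprint that turns Enhanced Input into navigation of two menu widgets on the viewport.
; BeginPlay adds the default mapping context and shows WBP_MainMenu; IA_Move steps the active widget's index, with a cooldown until the input completes.
; IA_Jump confirms by index to open levels, quit, or switch between the main menu and the WBP_MainMenu1 submenu.
; IA_B returns from the submenu, restoring the main menu's selection.
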(event `self.ReceiveBeginPlay`
  (bind _asplayer_controller (cast `PlayerController` (`self.GetController`)))
  (bind _returnvalue (pcsubsystem `EnhancedInputLocalPlayerSubsystem` _asplayer_controller))
  (`/Engine/EditorBlueprintResources/StandardMacros.IsValid` _returnvalue
    (:`Is Valid`
      (`EnhancedInputSubsystemInterface.AddMappingContext` _returnvalue "/Game/GAME/INPUT/IMC_Default.IMC_Default" 0 (struct))
      (bind _returnvalue_2 (`|CreateWidget` "/Game/GAME/BP/WBP/WBP_MainMenu.WBP_MainMenu_C"))
      (bind _output_get (set `self.Widget` _returnvalue_2))
      (`UserWidget.AddToViewport` _output_get 0))))

(event `EnhancedInput|/Game/GAME/INPUT/Actions/IA_Move`
  (params (ActionValue :type "Vector2D Structure") (ElapsedSeconds :type "Float (double-precision)") (TriggeredSeconds :type "Float (double-precision)") (InputAction :type "InputAction Object Reference" :default "/Game/GAME/INPUT/Actions/IA_Move.IA_Move"))
  (:`Triggered`
    (if (not (`self.cooldown`))
      (if (> ActionValue_Y 20.0)
        (set `self.cooldown` true)
        (if (`self.FirstMenu`)
          (`/Game/GAME/BP/WBP/WBP_MainMenu.ChangeIndex` (`self.Widget`) true)
          (else
            (`/Game/GAME/BP/WBP/WBP_MainMenu1.ChangeIndex` (`self.widget2`) true)))
        (elif (< ActionValue_Y -20.0)
          (set `self.cooldown` true)
          (if (`self.FirstMenu`)
            (`/Game/GAME/BP/WBP/WBP_MainMenu.ChangeIndex` (`self.Widget`) false)
            (else
              (`/Game/GAME/BP/WBP/WBP_MainMenu1.ChangeIndex` (`self.widget2`) false)))))))
  (:`Completed`
    (set `self.cooldown` false)))

(event `EnhancedInput|/Game/GAME/INPUT/Actions/IA_Jump`
  (params (ActionValue :type Boolean) (ElapsedSeconds :type "Float (double-precision)") (TriggeredSeconds :type "Float (double-precision)") (InputAction :type "InputAction Object Reference" :default "/Game/GAME/INPUT/Actions/IA_Jump.IA_Jump"))
  (bind _widget2 (`self.widget2`))
  (bind _widget (`self.Widget`))
  (:`Started`
    (if (`self.FirstMenu`)
      (switch `int` (`/Game/GAME/BP/WBP/WBP_MainMenu.Index` (`self.Widget`))
        (:`0`
          (`GameplayStatics.OpenLevelBySoftObjectPtr` "/Game/GAME/MAP/Level_02MAP.Level_02MAP"))
        (:`1`
          (`Widget.RemoveFromParent` (`self.Widget`))
          (bind _returnvalue (`|CreateWidget` "/Game/GAME/BP/WBP/WBP_MainMenu1.WBP_MainMenu1_C"))
          (bind _output_get (set `self.widget2` _returnvalue))
          (`UserWidget.AddToViewport` _output_get 0)
          (set `self.FirstMenu` false))
        (:`2`
          (`KismetSystemLibrary.QuitGame` null "Quit")))
      (else
        (switch `int` (`/Game/GAME/BP/WBP/WBP_MainMenu1.Index` _widget2)
          (:`0`
            (`GameplayStatics.OpenLevelBySoftObjectPtr` "/Game/GAME/MAP/Level_02MAP.Level_02MAP"))
          (:`1`
            (`GameplayStatics.OpenLevelBySoftObjectPtr` "/Game/GAME/MAP/Level_03MAP.Level_03MAP"))
          (:`2`
            (`Widget.RemoveFromParent` _widget2 :!label _label)
            (bind _returnvalue_2 (`|CreateWidget` "/Game/GAME/BP/WBP/WBP_MainMenu.WBP_MainMenu_C"))
            (bind _output_get_2 (set `self.Widget` _returnvalue_2))
            (`UserWidget.AddToViewport` _returnvalue_2 0)
            (`UserWidget.AddToViewport` _output_get_2 0)
            (set `self.FirstMenu` true)
            (set `/Game/GAME/BP/WBP/WBP_MainMenu.Index` 1 _widget)
            (`/Game/GAME/BP/WBP/WBP_MainMenu.UpddateVisual` _widget)))))))

(event `EnhancedInput|/Game/GAME/INPUT/Actions/IA_B`
  (params (ActionValue :type Boolean) (ElapsedSeconds :type "Float (double-precision)") (TriggeredSeconds :type "Float (double-precision)") (InputAction :type "InputAction Object Reference" :default "/Game/GAME/INPUT/Actions/IA_B.IA_B"))
  (:`Started`
    (if (not (`self.FirstMenu`))
      (goto _label))))

(fn `UserConstructionScript`)