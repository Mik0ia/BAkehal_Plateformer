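; BP_WaterZone is a water volume that reports to the level's Bp_WaterZoneManager when a player enters or leaves it.
; On BeginPlay it caches the first manager found, and the Hide flag chooses whether the Cube or the Dessus component is made invisible.
; Cube overlaps check the other actor for a BPC_Player component, then call PutIntoWater or RemoveFromWater on the manager, passing the zone itself.
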(event `self.ReceiveBeginPlay`
  (bind _outactors (`GameplayStatics.GetAllActorsOfClass` "/Game/GAME/BP/Manager/Bp_WaterZoneManager.Bp_WaterZoneManager_C"))
  (set `self.Manager` (`|GetArrayItem` _outactors))
  (if (`self.Hide`)
    (`SceneComponent.SetVisibility` (`self.Cube`) false false)
    (else
      (`SceneComponent.SetVisibility` (`self.Dessus`) false false))))

(event `self.Cube.OnComponentBeginOverlap`
  (params (OverlappedComponent :type "PrimitiveComponent Object Reference") (OtherActor :type "Actor Object Reference") (OtherComp :type "PrimitiveComponent Object Reference") (OtherBodyIndex :type Integer) (bFromSweep :type Boolean) (SweepResult :type "HitResult Structure (by ref)"))
  (`/Engine/EditorBlueprintResources/StandardMacros.IsValid` (`self.GetComponentByClass` OtherActor "/Game/GAME/BP/Components/BPC_Player.BPC_Player_C")
    (:`Is Valid`
      (`/Game/GAME/BP/Manager/Bp_WaterZoneManager.Put into Water` (`self.Manager`) self))))

(event `self.Cube.OnComponentEndOverlap`
  (params (OverlappedComponent :type "PrimitiveComponent Object Reference") (OtherActor :type "Actor Object Reference") (OtherComp :type "PrimitiveComponent Object Reference") (OtherBodyIndex :type Integer))
  (`/Engine/EditorBlueprintResources/StandardMacros.IsValid` (`self.GetComponentByClass` OtherActor "/Game/GAME/BP/Components/BPC_Player.BPC_Player_C")
    (:`Is Valid`
      (`/Game/GAME/BP/Manager/Bp_WaterZoneManager.Remove From Water` (`self.Manager`) self))))

(fn `UserConstructionScript`)