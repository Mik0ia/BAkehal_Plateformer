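; Trigger volume that switches the player's follow camera to a boss-fight view and wakes the boss.
; When the player enters the box, it sets CamBoss on the player, enables FollowPlayer on the first BP_Boss, and Tick eases the camera toward the Bp_BossCam transform until nearly equal.
; On exit it clears CamBoss and eases only the camera's rotation back to its initial value, leaving FollowPlayer set.
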(event `self.ReceiveBeginPlay`
  (bind _asbp_player (cast `/Game/GAME/BP/BP_Player` (`GameplayStatics.GetPlayerPawn` 0)))
  (set `self.As BP Player` _asbp_player)
  (bind _outactors (`GameplayStatics.GetAllActorsOfClass` "/Game/GAME/BP/Manager/Bp_BossCam.Bp_BossCam_C"))
  (set `self.CamBossRef` (`|GetArrayItem` _outactors)))

(event `self.ReceiveTick`
  (params (DeltaSeconds :type "Float (single-precision)"))
  (bind _as_bp_player (`self.As BP Player`))
  (bind _followcamera (`/Game/ThirdPerson/Blueprints/BP_ThirdPersonCharacter.FollowCamera` _as_bp_player))
  (bind _followcamera_2 (`/Game/ThirdPerson/Blueprints/BP_ThirdPersonCharacter.FollowCamera` (`self.As BP Player`)))
  (bind _caminitialrotation (`/Game/GAME/BP/BP_Player.CamInitialRotation` _as_bp_player))
  (bind _returnvalue (`SceneComponent.K2_GetComponentToWorld` (`/Game/GAME/BP/Manager/Bp_BossCam.Camera` (`self.CamBossRef`))))
  (bind _returnvalue_2 (`SceneComponent.K2_GetComponentRotation` _followcamera))
  (bind _returnvalue_3 (`SceneComponent.K2_GetComponentToWorld` _followcamera_2))
  (if (`self.Cam Boss Initialize`)
    (if (`KismetMathLibrary.NearlyEqual_TransformTransform` _returnvalue_3 _returnvalue 150.0 150.0 150.0)
      (set `self.Cam Boss Initialize` false)
      (else
        (`SceneComponent.K2_SetWorldTransform` _followcamera_2 (`KismetMathLibrary.TInterpTo` _returnvalue_3 _returnvalue (`GameplayStatics.GetWorldDeltaSeconds`) 7.0) false false)))
    (elif (`self.CamBossUnitialize`)
      (if (== _returnvalue_2 _caminitialrotation :`ErrorTolerance` 10.0)
        (set `self.CamBossUnitialize` false)
        (else
          (`SceneComponent.K2_SetWorldRotation` _followcamera (`KismetMathLibrary.RInterpTo` _returnvalue_2 _caminitialrotation (`GameplayStatics.GetWorldDeltaSeconds`) 7.0) false false))))))

(event `self.Box.OnComponentBeginOverlap`
  (params (OverlappedComponent :type "PrimitiveComponent Object Reference") (OtherActor :type "Actor Object Reference") (OtherComp :type "PrimitiveComponent Object Reference") (OtherBodyIndex :type Integer) (bFromSweep :type Boolean) (SweepResult :type "HitResult Structure (by ref)"))
  (if (== OtherActor (`self.As BP Player`))
    (if (not (`/Game/GAME/BP/BP_Player.Cam Boss ?` (`self.As BP Player`)))
      (`self.Cam Activate`))))

(event `self.Box.OnComponentEndOverlap`
  (params (OverlappedComponent :type "PrimitiveComponent Object Reference") (OtherActor :type "Actor Object Reference") (OtherComp :type "PrimitiveComponent Object Reference") (OtherBodyIndex :type Integer))
  (if (== OtherActor (`self.As BP Player`))
    (if (`/Game/GAME/BP/BP_Player.Cam Boss ?` (`self.As BP Player`))
      (`self.Cam Deactivate`))))

(event `Cam Activate`
  (set `/Game/GAME/BP/BP_Player.Cam Boss ?` true (`self.As BP Player`))
  (set `self.Cam Boss Initialize` true)
  (bind _outactors (`GameplayStatics.GetAllActorsOfClass` "/Game/GAME/BP/ENNEMY/BP_Boss.BP_Boss_C"))
  (set `/Game/GAME/BP/ENNEMY/BP_Boss.Follow Player` true (`|GetArrayItem` _outactors)))

(event `Cam Deactivate`
  (set `/Game/GAME/BP/BP_Player.Cam Boss ?` false (`self.As BP Player`))
  (set `self.CamBossUnitialize` true))

(fn `UserConstructionScript`)