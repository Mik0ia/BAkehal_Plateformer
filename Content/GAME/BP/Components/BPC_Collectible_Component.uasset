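; Actor component that keeps collected collectibles from respawning when a level is loaded again, enabled by CantRespawn.
; On a level's first setup, each owner adds a level-index and display-name key to BP_GameInstance, with a short delay before the level is flagged as set up.
; On later loads, owners without a substring-matched key destroy themselves.
; SupressInGI removes the owner's key from the GameInstance list.
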(event `self.ReceiveBeginPlay`
  (bind _returnvalue (`KismetSystemLibrary.GetDisplayName` (`self.GetOwner`)))
  (if (`self.Can'tRespawn`)
    (set `self.Finded` false)
    (`KismetSystemLibrary.Delay` 0.1)
    (bind _asbp_game_instance (cast `/Game/GAME/BP/BP_GameInstance` (`GameplayStatics.GetGameInstance`)))
    (bind _output_get (set `self.As BP Game Instance` _asbp_game_instance))
    (bind _collectiblehavebeensetup__ (`/Game/GAME/BP/BP_GameInstance.CollectibleHaveBeenSetup ?` _output_get))
    (bind _currentlevelindex (`/Game/GAME/BP/BP_GameInstance.CurrentLevelIndex` _output_get))
    (bind _output (`|GetArrayItem` _collectiblehavebeensetup__ _currentlevelindex))
    (if _output
      (bind _collectibleref (`/Game/GAME/BP/BP_GameInstance.CollectibleRef` _output_get))
      (for _array_element _collectibleref
        (bind _returnvalue_2 (`KismetStringLibrary.Concat_StrStr` "LV" (`KismetStringLibrary.Conv_IntToString` _currentlevelindex) "_"))
        (if (`KismetStringLibrary.Contains` _array_element _returnvalue_2)
          (if (`KismetStringLibrary.Contains` _array_element _returnvalue)
            (set `self.Finded` true)
            (break))))
      (if (not (`self.Finded`))
        (`Actor.K2_DestroyActor` (`self.GetOwner`)))
      (else
        (`KismetArrayLibrary.Array_Add` _collectibleref (`KismetStringLibrary.Concat_StrStr` _returnvalue_2 _returnvalue))
        (`KismetSystemLibrary.Delay` 0.1)
        (if (not _output)
          (`KismetArrayLibrary.Array_Set` _collectiblehavebeensetup__ _currentlevelindex true))))))

(event `SupressInGI`
  (bind _as_bp_game_instance (`self.As BP Game Instance`))
  (if (`self.Can'tRespawn`)
    (`KismetArrayLibrary.Array_RemoveItem` (`/Game/GAME/BP/BP_GameInstance.CollectibleRef` _as_bp_game_instance) (`KismetStringLibrary.Concat_StrStr` (`KismetStringLibrary.Concat_StrStr` "LV" (`KismetStringLibrary.Conv_IntToString` (`/Game/GAME/BP/BP_GameInstance.CurrentLevelIndex` _as_bp_game_instance)) "_") (`KismetSystemLibrary.GetDisplayName` (`self.GetOwner`))))))