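; Bp_Porte is a door actor that swings its mesh open and back in response to interaction events.
; On BeginPlay it stores the world rotation of StaticMesh5.
; Interact instantly adds a quarter turn of yaw to the mesh's current rotation, so repeated calls keep turning it.
; Uninteract snaps the mesh back to the stored rotation.
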(event `self.ReceiveBeginPlay`
  (set `self.World rotation` (`SceneComponent.K2_GetComponentRotation` (`self.StaticMesh5`))))

(event `/Game/GAME/BP/BPI_Interactable.Interact`
  (bind _staticmesh5 (`self.StaticMesh5`))
  (bind (_returnvalue_roll _returnvalue_pitch _returnvalue_yaw) (`KismetMathLibrary.BreakRotator` (`SceneComponent.K2_GetComponentRotation` _staticmesh5)))
  (`SceneComponent.K2_SetWorldRotation` _staticmesh5 (`KismetMathLibrary.MakeRotator` _returnvalue_roll _returnvalue_pitch (+ _returnvalue_yaw 90.0)) false false))

(event `/Game/GAME/BP/BPI_Uninteract.Uninteract`
  (`SceneComponent.K2_SetWorldRotation` (`self.StaticMesh5`) (`self.World rotation`) false false))

(fn `UserConstructionScript`)